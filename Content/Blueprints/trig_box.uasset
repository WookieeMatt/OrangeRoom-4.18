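; Trigger box actor that shows four text labels and signals the FPS_Character to open or close a gate.
; Begin overlap, only while NotInGame is true, reveals the texts and calls OpenGate on the overlapping character; end overlap always hides them and calls CloseGate.
; The hidetex event does the same hide and close without an overlap, using the first FPS_Character found in the world.
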(event `self.Box.OnComponentBeginOverlap`
  (params (OverlappedComponent :type "PrimitiveComponent Object Reference") (OtherActor :type "Actor Object Reference") (OtherComp :type "PrimitiveComponent Object Reference") (OtherBodyIndex :type Integer) (bFromSweep :type Boolean) (SweepResult :type "HitResult Structure (by ref)"))
  (if (`self.not in game`)
    (bind _asfps_character (cast `/Game/Blueprints/FPS_Character` OtherActor))
    (`SceneComponent.SetVisibility` (`self.TextRender1`) true false)
    (`SceneComponent.SetVisibility` (`self.TextRender`) true false)
    (`SceneComponent.SetVisibility` (`self.TextRender3`) true false)
    (`SceneComponent.SetVisibility` (`self.TextRender2`) true false)
    (`/Game/Blueprints/FPS_Character.open gate` _asfps_character)))

(event `self.Box.OnComponentEndOverlap`
  (params (OverlappedComponent :type "PrimitiveComponent Object Reference") (OtherActor :type "Actor Object Reference") (OtherComp :type "PrimitiveComponent Object Reference") (OtherBodyIndex :type Integer))
  (bind _asfps_character (cast `/Game/Blueprints/FPS_Character` OtherActor))
  (`SceneComponent.SetVisibility` (`self.TextRender1`) false false)
  (`SceneComponent.SetVisibility` (`self.TextRender`) false false)
  (`SceneComponent.SetVisibility` (`self.TextRender3`) false false)
  (`SceneComponent.SetVisibility` (`self.TextRender2`) false false)
  (`/Game/Blueprints/FPS_Character.close gate` _asfps_character))

(event `hide tex`
  (bind _outactors (`GameplayStatics.GetAllActorsOfClass` "/Game/Blueprints/FPS_Character.FPS_Character_C"))
  (`SceneComponent.SetVisibility` (`self.TextRender1`) false false)
  (`SceneComponent.SetVisibility` (`self.TextRender`) false false)
  (`SceneComponent.SetVisibility` (`self.TextRender3`) false false)
  (`SceneComponent.SetVisibility` (`self.TextRender2`) false false)
  (`/Game/Blueprints/FPS_Character.close gate` (`KismetArrayLibrary.Array_Get` _outactors)))

(fn `UserConstructionScript`)