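; Special bonus bubble actor that plays a start sound on spawn, drifts upward each tick and destroys itself after seven seconds.
; Any overlap with its Sphere1 component destroys it, plays a bonus sound, and increments the first FPS_Character's hit count while granting extra balls.
; The rise is a fixed per-frame offset, so its speed depends on frame rate.
; A timeline meant to wobble the sphere's scale is never triggered.
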(event `self.Sphere1.OnComponentBeginOverlap`
  (params (OverlappedComponent :type "PrimitiveComponent Object Reference") (OtherActor :type "Actor Object Reference") (OtherComp :type "PrimitiveComponent Object Reference") (OtherBodyIndex :type Integer) (bFromSweep :type Boolean) (SweepResult :type "HitResult Structure (by ref)"))
  ;[1 1 1] hit by ball
  (`self.K2_DestroyActor`)
  (`GameplayStatics.PlaySoundAtLocation` "/Game/Audio/Bonus_.Bonus_" (`self.K2_GetActorLocation`))
  (bind _outactors (`GameplayStatics.GetAllActorsOfClass` "/Game/Blueprints/FPS_Character.FPS_Character_C"))
  (bind _item (`KismetArrayLibrary.Array_Get` _outactors))
  (set `/Game/Blueprints/FPS_Character.bubble hit number` (+ (`/Game/Blueprints/FPS_Character.bubble hit number` _item) 1) _item)
  (set `/Game/Blueprints/FPS_Character.ball number` (+ (`/Game/Blueprints/FPS_Character.ball number` _item) 40) _item))

(event `self.ReceiveBeginPlay`
  ;[1 1 1] hit by ball and play spec sound when start
  (`GameplayStatics.PlaySoundAtLocation` "/Game/Audio/bonus_start.bonus_start" (`self.K2_GetActorLocation`)) ; Play firing sound
  (`KismetSystemLibrary.Delay` 7.0)
  (`self.K2_DestroyActor`))

(event `self.ReceiveTick`
  (params (DeltaSeconds :type "Float (single-precision)"))
  ;[1 1 1] raise the ball to top
  (`SceneComponent.K2_AddRelativeLocation` (`self.DefaultSceneRoot`) (0.0 0.0 0.2) false false))

(fn `UserConstructionScript`)